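; BP_TronPlayerCharacter is a player character Blueprint that supplies movement and look input and toggles weapons by tag.
; SetWeaponAsset unequips when the current weapon already has the exact tag, otherwise it equips the first matching asset from BPWeaponAssetManager with a blend space transition.
; GetMovementInput and GetRotationInput convert the IA_Move and IA_Look values into movement and rotation values.
; The event graph holds only disabled stub events and unused weapon lookup nodes.
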(event `Key|One`
  (params (Key :type "Key Structure")))

(event `Key|Two`
  (params (Key :type "Key Structure")))

(fn `GetMovementInput`
  (returns (ReturnValue :type "Vector Structure"))
  (bind (_returnvalue_x _returnvalue_y) (`KismetMathLibrary.BreakVector2D` (`|GetInputActionValue`)))
  (return (`KismetMathLibrary.MakeVector` _returnvalue_x _returnvalue_y)))

(fn `GetRotationInput`
  (returns (ReturnValue :type "Rotator Structure"))
  (bind (_returnvalue_x _returnvalue_y) (`KismetMathLibrary.BreakVector2D` (`|GetInputActionValue`)))
  (return (`KismetMathLibrary.MakeRotator` _returnvalue_y _returnvalue_x)))

(fn `SetWeaponAsset`
  (params (Tag :type "GameplayTag Structure"))
  (if (`BlueprintGameplayTagLibrary.HasTag` (`WeaponComponent.GetCurrentWeaponTags` (`self.WeaponComponent`)) Tag true)
    (`self.UnequipWeapon`)
    (else
      (`self.EquipWeapon` (`|GetArrayItem` (`TronRpgWeaponAssetManager.GetWeaponsByTag` (subsystem `/Game/Data/Weapon/BP_WeaponAssetManager`) Tag))))))

(fn `UserConstructionScript`)